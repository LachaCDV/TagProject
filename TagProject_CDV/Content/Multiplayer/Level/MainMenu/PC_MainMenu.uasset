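; PC_MainMenu is a main menu player controller Blueprint whose logic is currently disconnected, with an empty BeginPlay and construction script.
; An unwired chain would create WB_MainMenu for the local controller, show the mouse cursor and, on authority, call SpawnCharacter on GI_SteamTagProject.
; A second unwired chain calls SpawnCharacter through BP_GameInstance instead.
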(event EventBeginPlay)

(fn ConstructionScript)