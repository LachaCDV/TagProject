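; Game mode for a tag game that tracks joining players.
; On PostLogin it adds the new controller to an array and prints its display name.
; A disconnected FlipFlop branch would alternate spawning and possessing default and red third-person characters, but it never runs.
; A helper function supplies that branch with the transform of a randomly chosen PlayerStart.
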(event EventBeginPlay)

(event EventTick
  (params (DeltaSeconds :type Float%20%28single-precision%29)))

(event EventPostLogin
  (params (NewPlayer :type Player%20Controller%20Object%20Reference))
  (Utilities|Array|Add (Variables|Default|GetNew%20Player) NewPlayer)
  (Development|PrintString (Utilities|GetDisplayName NewPlayer)))

(fn ConstructionScript)

(fn GetRandomPlayerStart
  (bind _outactors (Actor|GetAllActorsOfClass "/Script/Engine.PlayerStart"))
  (return (Transformation|GetActorTransform (Utilities|Array|Get(acopy) _outactors (Math|Random|RandomIntegerinRange 0 (- (Utilities|Array|Length _outactors) 1))))))